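; Game manager for a shogi-style board game with separate move and attack actions, running two-player turns through a phase state machine.
; Click events route by phase to move or attack resolution, while Tick switches turns at End and resets action flags at Standby.
; CheckKomaRange expands direction patterns, including knight jumps and blockable sliding rays, into empty and occupied cells on a flat 81-cell board.
; CheckRadiateGrid flags those cells for highlighting and click validation.
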(event Custom|ChangedMovingPhase
  (bind _selectedkoma (Variables|Default|GetselectedKoma))
  ;[1 1 1] AttackPhaseになった直後に呼ぶイベント
  (if (Utilities|IsValid _selectedkoma)
    (Utilities|Array|Clear (Variables|Default|GetkomaRangeList))
    (Utilities|Array|Clear (Variables|Default|GetblockGridList))
    (CallFunction|CheckKomaRange _selectedkoma (Variables|/Game/ブループリント/koma/koma_BP.koma_BP_C|GetmoveRange _selectedkoma)) ; 選択された駒が動ける範囲を取得する
    (CallFunction|CheckRadiateGrid) ; 移動範囲を見てグリッドを光らせる
  ))

(event Custom|SelectedKoma_Event
  (params (koma :type Koma%20BP%20Object%20Reference))
  ;[1 1 1] 駒クリック時に呼ばれる
  (switch Utilities|FlowControl|Switch|SwitchonPhase (Variables|Default|GetcurrentPhase)
    (:NewEnumerator1
      (CallFunction|PhaseChange "NewEnumerator7"))
    (:NewEnumerator5
      (CallFunction|InAttackRange (Utilities|Array|Get(acopy) (Variables|Default|GetgridList) (Variables|/Game/ブループリント/koma/koma_BP.koma_BP_C|GetgridIndex koma))))))

(event Custom|ChangeAttackPhase
  (bind _selectedkoma (Variables|Default|GetselectedKoma))
  ;[1 1 1] MovingPhaseになった直後に呼ぶイベント
  (if (Utilities|IsValid _selectedkoma)
    (Utilities|Array|Clear (Variables|Default|GetkomaRangeList))
    (Utilities|Array|Clear (Variables|Default|GetblockGridList))
    (CallFunction|CheckKomaRange _selectedkoma (Variables|/Game/ブループリント/koma/koma_BP.koma_BP_C|GetattackRange _selectedkoma)) ; 選択された駒が動ける範囲を取得する
    (CallFunction|CheckRadiateGrid) ; 範囲を見てグリッドを光らせる
  ))

(event Custom|SelectedGrid_Event
  (params (grid :type Grid%20BP%20Object%20Reference))
  ;[1 1 1] グリッドをクリックしたとき
  ;[1 1 1] 駒の移動、攻撃処理
  (switch Utilities|FlowControl|Switch|SwitchonPhase (Variables|Default|GetcurrentPhase)
    (:NewEnumerator7
      (CallFunction|PhaseChange "NewEnumerator1")
      (Variables|Default|SetselectedKoma 0))
    (:NewEnumerator4
      ;;[1 1 1] 移動処理
      (CallFunction|InMovingRange grid))
    (:NewEnumerator5
      ;;[1 1 1] 攻撃処理
      (CallFunction|InAttackRange grid))))

(event EventBeginPlay
  (CallFunction|TurnChange "NewEnumerator0")
  (CallFunction|PhaseChange "NewEnumerator1"))

(event EventTick
  (params (DeltaSeconds :type Float%20%28single-precision%29))
  ;[1 1 1] フェイズ分岐
  (switch Utilities|FlowControl|Switch|SwitchonPhase (Variables|Default|GetcurrentPhase)
    (:NewEnumerator0
      ;[1 1 1] フラグを全てリセットしてMainへ
      (Variables|Default|SetisAttack false)
      (Variables|Default|SetisMoving false)
      (CallFunction|PhaseChange "NewEnumerator1"))
    (:NewEnumerator6
      ;[1 1 1] 現在特にチェックすることはないので即切り替え
      (switch Utilities|FlowControl|Switch|SwitchonTurn (Variables|Default|GetcurrentTurn)
        (:NewEnumerator0
          (CallFunction|TurnChange "NewEnumerator1"))
        (:NewEnumerator1
          (CallFunction|TurnChange "NewEnumerator0")))
      (CallFunction|PhaseChange "NewEnumerator0"))))

(fn ConstructionScript
  ;[1 1 1] グリッドを受け入れる準備
  (Utilities|Array|Resize (Variables|Default|GetgridList) 81)
  ;[1 1 1] 駒達を位置順に格納する準備
  (Utilities|Array|Resize (Variables|Default|GetcurrentKomaPositionList) 81))

(fn CheckKomaRange
  (params (koma :type Koma%20BP%20Object%20Reference) (range :type Set%20of%20Range%20Enums :default "NewEnumerator4"))
  (bind _direction (Variables|/Game/ブループリント/koma/koma_BP.koma_BP_C|Getdirection koma))
  (bind _gridposition (Variables|/Game/ブループリント/koma/koma_BP.koma_BP_C|GetgridPosition koma))
  (bind _gridposition_2 (Variables|/Game/ブループリント/koma/koma_BP.koma_BP_C|GetgridPosition koma))
  (bind _gridposition_3 (Variables|/Game/ブループリント/koma/koma_BP.koma_BP_C|GetgridPosition koma))
  (bind _gridposition_4 (Variables|/Game/ブループリント/koma/koma_BP.koma_BP_C|GetgridPosition koma))
  (bind _gridposition_5 (Variables|/Game/ブループリント/koma/koma_BP.koma_BP_C|GetgridPosition koma))
  (bind _gridposition_6 (Variables|/Game/ブループリント/koma/koma_BP.koma_BP_C|GetgridPosition koma))
  (bind _gridposition_7 (Variables|/Game/ブループリント/koma/koma_BP.koma_BP_C|GetgridPosition koma))
  (bind _gridposition_8 (Variables|/Game/ブループリント/koma/koma_BP.koma_BP_C|GetgridPosition koma))
  (bind _gridposition_9 (Variables|/Game/ブループリント/koma/koma_BP.koma_BP_C|GetgridPosition koma))
  (bind _gridposition_10 (Variables|/Game/ブループリント/koma/koma_BP.koma_BP_C|GetgridPosition koma))
  (bind _gridposition_11 (Variables|/Game/ブループリント/koma/koma_BP.koma_BP_C|GetgridPosition koma))
  (bind _gridposition_12 (Variables|/Game/ブループリント/koma/koma_BP.koma_BP_C|GetgridPosition koma))
  (bind _gridposition_13 (Variables|/Game/ブループリント/koma/koma_BP.koma_BP_C|GetgridPosition koma))
  (bind _gridposition_14 (Variables|/Game/ブループリント/koma/koma_BP.koma_BP_C|GetgridPosition koma))
  (bind _direction_2 (Variables|/Game/ブループリント/koma/koma_BP.koma_BP_C|Getdirection koma))
  (bind _direction_3 (Variables|/Game/ブループリント/koma/koma_BP.koma_BP_C|Getdirection koma))
  (bind _direction_4 (Variables|/Game/ブループリント/koma/koma_BP.koma_BP_C|Getdirection koma))
  (bind _direction_5 (Variables|/Game/ブループリント/koma/koma_BP.koma_BP_C|Getdirection koma))
  (bind _direction_6 (Variables|/Game/ブループリント/koma/koma_BP.koma_BP_C|Getdirection koma))
  (bind _gridposition_15 (Variables|/Game/ブループリント/koma/koma_BP.koma_BP_C|GetgridPosition koma))
  (bind _gridposition_16 (Variables|/Game/ブループリント/koma/koma_BP.koma_BP_C|GetgridPosition koma))
  (bind _gridposition_17 (Variables|/Game/ブループリント/koma/koma_BP.koma_BP_C|GetgridPosition koma))
  (bind _gridposition_18 (Variables|/Game/ブループリント/koma/koma_BP.koma_BP_C|GetgridPosition koma))
  (bind _gridposition_19 (Variables|/Game/ブループリント/koma/koma_BP.koma_BP_C|GetgridPosition koma))
  (bind _gridposition_20 (Variables|/Game/ブループリント/koma/koma_BP.koma_BP_C|GetgridPosition koma))
  (bind _gridposition_21 (Variables|/Game/ブループリント/koma/koma_BP.koma_BP_C|GetgridPosition koma))
  (bind _gridposition_22 (Variables|/Game/ブループリント/koma/koma_BP.koma_BP_C|GetgridPosition koma))
  (bind _gridposition_23 (Variables|/Game/ブループリント/koma/koma_BP.koma_BP_C|GetgridPosition koma))
  (bind _gridposition_24 (Variables|/Game/ブループリント/koma/koma_BP.koma_BP_C|GetgridPosition koma))
  (bind _gridposition_25 (Variables|/Game/ブループリント/koma/koma_BP.koma_BP_C|GetgridPosition koma))
  (bind _gridposition_26 (Variables|/Game/ブループリント/koma/koma_BP.koma_BP_C|GetgridPosition koma))
  (bind _gridposition_27 (Variables|/Game/ブループリント/koma/koma_BP.koma_BP_C|GetgridPosition koma))
  (bind _gridposition_28 (Variables|/Game/ブループリント/koma/koma_BP.koma_BP_C|GetgridPosition koma))
  ;[1 1 1] 移動範囲を渡されたRangeから作成
  (bind _result (Utilities|Set|ToArray range))
  (for _array_element _result
    (switch Utilities|FlowControl|Switch|SwitchonRange _array_element
      (:NewEnumerator4
        ;[1 1 1] 正面
        (LocalVariables|Setpoint (Utilities|Struct|MakeIntPoint (+ (* (Variables|/Game/ブループリント/koma/koma_BP.koma_BP_C|Getdirection koma) 1) (.x _gridposition)) (.y _gridposition)))
        (CallFunction|CheckUseGrid (LocalVariables|Getpoint)))
      (:NewEnumerator5
        ;[1 1 1] 右正面
        (LocalVariables|Setpoint (Utilities|Struct|MakeIntPoint (+ (.x _gridposition_2) (* _direction_2 1)) (+ (.y _gridposition_2) (* _direction_2 1))))
        (CallFunction|CheckUseGrid (LocalVariables|Getpoint)))
      (:NewEnumerator6
        ;[1 1 1] 右
        (LocalVariables|Setpoint (Utilities|Struct|MakeIntPoint (.x _gridposition_3) (+ (.y _gridposition_3) (* (Variables|/Game/ブループリント/koma/koma_BP.koma_BP_C|Getdirection koma) 1))))
        (CallFunction|CheckUseGrid (LocalVariables|Getpoint)))
      (:NewEnumerator3
        ;[1 1 1] 右後ろ
        (LocalVariables|Setpoint (Utilities|Struct|MakeIntPoint (- (.x _gridposition_5) (* _direction_6 1)) (+ (.y _gridposition_5) (* _direction_6 1))))
        (CallFunction|CheckUseGrid (LocalVariables|Getpoint)))
      (:NewEnumerator7
        ;[1 1 1] 後ろ
        (LocalVariables|Setpoint (Utilities|Struct|MakeIntPoint (- (.x _gridposition_8) (* (Variables|/Game/ブループリント/koma/koma_BP.koma_BP_C|Getdirection koma) 1)) (.y _gridposition_8)))
        (CallFunction|CheckUseGrid (LocalVariables|Getpoint)))
      (:NewEnumerator8
        ;[1 1 1] 左後ろ
        (LocalVariables|Setpoint (Utilities|Struct|MakeIntPoint (- (.x _gridposition_10) (* _direction_3 1)) (- (.y _gridposition_10) (* _direction_3 1))))
        (CallFunction|CheckUseGrid (LocalVariables|Getpoint)))
      (:NewEnumerator9
        ;[1 1 1] 左
        (LocalVariables|Setpoint (Utilities|Struct|MakeIntPoint (.x _gridposition_9) (- (.y _gridposition_9) (* (Variables|/Game/ブループリント/koma/koma_BP.koma_BP_C|Getdirection koma) 1))))
        (CallFunction|CheckUseGrid (LocalVariables|Getpoint)))
      (:NewEnumerator10
        ;[1 1 1] 左正面
        (LocalVariables|Setpoint (Utilities|Struct|MakeIntPoint (+ (.x _gridposition_6) (* _direction_5 1)) (- (.y _gridposition_6) (* _direction_5 1))))
        (CallFunction|CheckUseGrid (LocalVariables|Getpoint)))
      (:NewEnumerator11
        ;[1 1 1] 桂馬右
        (LocalVariables|Setpoint (Utilities|Struct|MakeIntPoint (+ (.x _gridposition_12) (* _direction_4 2)) (+ (.y _gridposition_12) (* _direction_4 1))))
        (CallFunction|CheckUseGrid (LocalVariables|Getpoint)))
      (:NewEnumerator12
        ;[1 1 1] 桂馬左
        (LocalVariables|Setpoint (Utilities|Struct|MakeIntPoint (+ (.x _gridposition_16) (* _direction 2)) (- (.y _gridposition_16) (* _direction 1))))
        (CallFunction|CheckUseGrid (LocalVariables|Getpoint)))
      (:NewEnumerator15
        ;[1 1 1] 香車
        (bind _index (Utilities|FlowControl|ForLoopwithBreak 1 (Variables|Default|GetBoardHeight) :!label _label)
          (:LoopBody
            (LocalVariables|Setpoint (Utilities|Struct|MakeIntPoint (+ (.x _gridposition_13) (* _index (Variables|/Game/ブループリント/koma/koma_BP.koma_BP_C|Getdirection koma))) (.y _gridposition_13)))
            (CallFunction|CheckUseGrid (LocalVariables|Getpoint))
            (if (Utilities|IsValid (Utilities|Array|Get(acopy) (Variables|Default|GetcurrentKomaPositionList) (Utilities|PointtoGridIndex (LocalVariables|Getpoint))))
              (goto _label Break)))))
      (:NewEnumerator13
        ;[1 1 1] 飛車
        (Utilities|FlowControl|Sequence
          (:then_0
            ;;[1 1 1] 前
            (bind _index_2 (Utilities|FlowControl|ForLoopwithBreak 1 (Variables|Default|GetBoardHeight) :!label _label_2)
              (:LoopBody
                (bind _output_get (LocalVariables|Setpoint (Utilities|Struct|MakeIntPoint (+ (.x _gridposition_25) _index_2) (.y _gridposition_25))))
                (CallFunction|CheckUseGrid (LocalVariables|Getpoint))
                (if (Utilities|IsValid (Utilities|Array|Get(acopy) (Variables|Default|GetcurrentKomaPositionList) (Utilities|PointtoGridIndex _output_get)))
                  (goto _label_2 Break)))))
          (:then_1
            ;;[1 1 1] 右
            (bind _index_3 (Utilities|FlowControl|ForLoopwithBreak 1 (Variables|Default|GetBoardHeight) :!label _label_3)
              (:LoopBody
                (bind _output_get_2 (LocalVariables|Setpoint (Utilities|Struct|MakeIntPoint (.x _gridposition_26) (+ (.y _gridposition_26) _index_3))))
                (CallFunction|CheckUseGrid (LocalVariables|Getpoint))
                (if (Utilities|IsValid (Utilities|Array|Get(acopy) (Variables|Default|GetcurrentKomaPositionList) (Utilities|PointtoGridIndex _output_get_2)))
                  (goto _label_3 Break)))))
          (:then_2
            ;;[1 1 1] 後ろ
            (bind _index_4 (Utilities|FlowControl|ForLoopwithBreak 1 (Variables|Default|GetBoardHeight) :!label _label_4)
              (:LoopBody
                (bind _output_get_3 (LocalVariables|Setpoint (Utilities|Struct|MakeIntPoint (- (.x _gridposition_27) _index_4) (.y _gridposition_27))))
                (CallFunction|CheckUseGrid (LocalVariables|Getpoint))
                (if (Utilities|IsValid (Utilities|Array|Get(acopy) (Variables|Default|GetcurrentKomaPositionList) (Utilities|PointtoGridIndex _output_get_3)))
                  (goto _label_4 Break)))))
          (:then_3
            ;;[1 1 1] 左
            (bind _index_5 (Utilities|FlowControl|ForLoopwithBreak 1 (Variables|Default|GetBoardHeight) :!label _label_5)
              (:LoopBody
                (bind _output_get_4 (LocalVariables|Setpoint (Utilities|Struct|MakeIntPoint (.x _gridposition_28) (- (.y _gridposition_28) _index_5))))
                (CallFunction|CheckUseGrid (LocalVariables|Getpoint))
                (if (Utilities|IsValid (Utilities|Array|Get(acopy) (Variables|Default|GetcurrentKomaPositionList) (Utilities|PointtoGridIndex _output_get_4)))
                  (goto _label_5 Break)))))))
      (:NewEnumerator14
        ;[1 1 1] 角行
        (Utilities|FlowControl|Sequence
          (:then_0
            ;;[1 1 1] 右上
            (bind _index_6 (Utilities|FlowControl|ForLoopwithBreak 1 (Variables|Default|GetBoardHeight) :!label _label_6)
              (:LoopBody
                (bind _output_get_5 (LocalVariables|Setpoint (Utilities|Struct|MakeIntPoint (+ (.x _gridposition_21) _index_6) (+ (.y _gridposition_21) _index_6))))
                (CallFunction|CheckUseGrid (LocalVariables|Getpoint))
                (if (Utilities|IsValid (Utilities|Array|Get(acopy) (Variables|Default|GetcurrentKomaPositionList) (Utilities|PointtoGridIndex _output_get_5)))
                  (goto _label_6 Break)))))
          (:then_1
            ;;[1 1 1] 左上
            (bind _index_7 (Utilities|FlowControl|ForLoopwithBreak 1 (Variables|Default|GetBoardHeight) :!label _label_7)
              (:LoopBody
                (bind _output_get_6 (LocalVariables|Setpoint (Utilities|Struct|MakeIntPoint (+ (.x _gridposition_22) _index_7) (- (.y _gridposition_22) _index_7))))
                (CallFunction|CheckUseGrid (LocalVariables|Getpoint))
                (if (Utilities|IsValid (Utilities|Array|Get(acopy) (Variables|Default|GetcurrentKomaPositionList) (Utilities|PointtoGridIndex _output_get_6)))
                  (goto _label_7 Break)))))
          (:then_2
            ;;[1 1 1] 左上
            (bind _index_8 (Utilities|FlowControl|ForLoopwithBreak 1 (Variables|Default|GetBoardHeight) :!label _label_8)
              (:LoopBody
                (bind _output_get_7 (LocalVariables|Setpoint (Utilities|Struct|MakeIntPoint (- (.x _gridposition_23) _index_8) (+ (.y _gridposition_23) _index_8))))
                (CallFunction|CheckUseGrid (LocalVariables|Getpoint))
                (if (Utilities|IsValid (Utilities|Array|Get(acopy) (Variables|Default|GetcurrentKomaPositionList) (Utilities|PointtoGridIndex _output_get_7)))
                  (goto _label_8 Break)))))
          (:then_3
            ;;[1 1 1] 左上
            (bind _index_9 (Utilities|FlowControl|ForLoopwithBreak 1 (Variables|Default|GetBoardHeight) :!label _label_9)
              (:LoopBody
                (bind _output_get_8 (LocalVariables|Setpoint (Utilities|Struct|MakeIntPoint (- (.x _gridposition_24) _index_9) (- (.y _gridposition_24) _index_9))))
                (CallFunction|CheckUseGrid (LocalVariables|Getpoint))
                (if (Utilities|IsValid (Utilities|Array|Get(acopy) (Variables|Default|GetcurrentKomaPositionList) (Utilities|PointtoGridIndex _output_get_8)))
                  (goto _label_9 Break)))))))
      (:NewEnumerator16
        ;[1 1 1] 飛車攻撃範囲
        (Utilities|FlowControl|Sequence
          (:then_0
            ;;[1 1 1] 前
            (bind _index_10 (Utilities|FlowControl|ForLoopwithBreak 1 2 :!label _label_10)
              (:LoopBody
                (bind _output_get_9 (LocalVariables|Setpoint (Utilities|Struct|MakeIntPoint (+ (.x _gridposition_18) _index_10) (.y _gridposition_18))))
                (CallFunction|CheckUseGrid (LocalVariables|Getpoint))
                (if (Utilities|IsValid (Utilities|Array|Get(acopy) (Variables|Default|GetcurrentKomaPositionList) (Utilities|PointtoGridIndex _output_get_9)))
                  (goto _label_10 Break)))))
          (:then_1
            ;;[1 1 1] 右
            (bind _index_11 (Utilities|FlowControl|ForLoopwithBreak 1 2 :!label _label_11)
              (:LoopBody
                (bind _output_get_10 (LocalVariables|Setpoint (Utilities|Struct|MakeIntPoint (.x _gridposition_20) (+ (.y _gridposition_20) _index_11))))
                (CallFunction|CheckUseGrid (LocalVariables|Getpoint))
                (if (Utilities|IsValid (Utilities|Array|Get(acopy) (Variables|Default|GetcurrentKomaPositionList) (Utilities|PointtoGridIndex _output_get_10)))
                  (goto _label_11 Break)))))
          (:then_2
            ;;[1 1 1] 後ろ
            (bind _index_12 (Utilities|FlowControl|ForLoopwithBreak 1 2 :!label _label_12)
              (:LoopBody
                (bind _output_get_11 (LocalVariables|Setpoint (Utilities|Struct|MakeIntPoint (- (.x _gridposition_4) _index_12) (.y _gridposition_4))))
                (CallFunction|CheckUseGrid (LocalVariables|Getpoint))
                (if (Utilities|IsValid (Utilities|Array|Get(acopy) (Variables|Default|GetcurrentKomaPositionList) (Utilities|PointtoGridIndex _output_get_11)))
                  (goto _label_12 Break)))))
          (:then_3
            ;;[1 1 1] 左
            (bind _index_13 (Utilities|FlowControl|ForLoopwithBreak 1 2 :!label _label_13)
              (:LoopBody
                (bind _output_get_12 (LocalVariables|Setpoint (Utilities|Struct|MakeIntPoint (.x _gridposition_19) (- (.y _gridposition_19) _index_13))))
                (CallFunction|CheckUseGrid (LocalVariables|Getpoint))
                (if (Utilities|IsValid (Utilities|Array|Get(acopy) (Variables|Default|GetcurrentKomaPositionList) (Utilities|PointtoGridIndex _output_get_12)))
                  (goto _label_13 Break)))))))
      (:NewEnumerator17
        ;[1 1 1] 角行攻撃範囲
        (Utilities|FlowControl|Sequence
          (:then_0
            ;;[1 1 1] 右上
            (bind _index_14 (Utilities|FlowControl|ForLoopwithBreak 1 2 :!label _label_14)
              (:LoopBody
                (bind _output_get_13 (LocalVariables|Setpoint (Utilities|Struct|MakeIntPoint (+ (.x _gridposition_17) _index_14) (+ (.y _gridposition_17) _index_14))))
                (CallFunction|CheckUseGrid (LocalVariables|Getpoint))
                (if (Utilities|IsValid (Utilities|Array|Get(acopy) (Variables|Default|GetcurrentKomaPositionList) (Utilities|PointtoGridIndex _output_get_13)))
                  (goto _label_14 Break)))))
          (:then_1
            ;;[1 1 1] 左上
            (bind _index_15 (Utilities|FlowControl|ForLoopwithBreak 1 2 :!label _label_15)
              (:LoopBody
                (bind _output_get_14 (LocalVariables|Setpoint (Utilities|Struct|MakeIntPoint (+ (.x _gridposition_7) _index_15) (- (.y _gridposition_7) _index_15))))
                (CallFunction|CheckUseGrid (LocalVariables|Getpoint))
                (if (Utilities|IsValid (Utilities|Array|Get(acopy) (Variables|Default|GetcurrentKomaPositionList) (Utilities|PointtoGridIndex _output_get_14)))
                  (goto _label_15 Break)))))
          (:then_2
            ;;[1 1 1] 左上
            (bind _index_16 (Utilities|FlowControl|ForLoopwithBreak 1 2 :!label _label_16)
              (:LoopBody
                (bind _output_get_15 (LocalVariables|Setpoint (Utilities|Struct|MakeIntPoint (- (.x _gridposition_11) _index_16) (+ (.y _gridposition_11) _index_16))))
                (CallFunction|CheckUseGrid (LocalVariables|Getpoint))
                (if (Utilities|IsValid (Utilities|Array|Get(acopy) (Variables|Default|GetcurrentKomaPositionList) (Utilities|PointtoGridIndex _output_get_15)))
                  (goto _label_16 Break)))))
          (:then_3
            ;;[1 1 1] 左上
            (bind _index_17 (Utilities|FlowControl|ForLoopwithBreak 1 2 :!label _label_17)
              (:LoopBody
                (bind _output_get_16 (LocalVariables|Setpoint (Utilities|Struct|MakeIntPoint (- (.x _gridposition_14) _index_17) (- (.y _gridposition_14) _index_17))))
                (CallFunction|CheckUseGrid (LocalVariables|Getpoint))
                (if (Utilities|IsValid (Utilities|Array|Get(acopy) (Variables|Default|GetcurrentKomaPositionList) (Utilities|PointtoGridIndex _output_get_16)))
                  (goto _label_17 Break)))))))
      (:NewEnumerator18
        ;[1 1 1] 香車
        (bind _index_18 (Utilities|FlowControl|ForLoopwithBreak 1 2 :!label _label_18)
          (:LoopBody
            (LocalVariables|Setpoint (Utilities|Struct|MakeIntPoint (+ (.x _gridposition_15) (* _index_18 (Variables|/Game/ブループリント/koma/koma_BP.koma_BP_C|Getdirection koma))) (.y _gridposition_15)))
            (CallFunction|CheckUseGrid (LocalVariables|Getpoint))
            (if (Utilities|IsValid (Utilities|Array|Get(acopy) (Variables|Default|GetcurrentKomaPositionList) (Utilities|PointtoGridIndex (LocalVariables|Getpoint))))
              (goto _label_18 Break)))))))
  (return))

(fn CheckRadiateGrid
  (Utilities|FlowControl|Sequence
    (:then_0
      ;[1 1 1] 範囲内のグリッド
      (Utilities|Array|Clear (Variables|Default|GetinRangeGridList))
      (for _array_element (Variables|Default|GetkomaRangeList)
        ;;[1 1 1] 駒が実際に移動、攻撃できるグリッドのリスト
        (Utilities|Array|Add (Variables|Default|GetinRangeGridList) (Utilities|Array|Get(acopy) (Variables|Default|GetgridList) (Utilities|PointtoGridIndex _array_element)))
        (Utilities|IsValid (Utilities|Array|Get(acopy) (Variables|Default|GetgridList) (Utilities|PointtoGridIndex _array_element))
          (:Is%20Valid
            (Variables|/Game/Grid_BP.Grid_BP_C|SetisRange (Utilities|Array|Get(acopy) (Variables|Default|GetgridList) (Utilities|PointtoGridIndex _array_element)) true)))))
    (:then_1
      ;[1 1 1] いけないグリッド
      (for _array_element_2 (Variables|Default|GetblockGridList)
        (Utilities|Array|Add (Variables|Default|GetcurrentBlockGridList) (Utilities|Array|Get(acopy) (Variables|Default|GetgridList) (Utilities|PointtoGridIndex _array_element_2)))
        (Variables|/Game/Grid_BP.Grid_BP_C|SetisBlock (Utilities|Array|Get(acopy) (Variables|Default|GetgridList) (Utilities|PointtoGridIndex _array_element_2)) true)))))

(fn CheckUseGrid
  (params (point :type Int%20Point%20Structure))
  (bind (_x _y) (Utilities|Struct|BreakIntPoint point))
  (bind _boardheight (Variables|Default|GetBoardHeight))
  ;[1 1 1] 移動先がボード外ではないか
  (if (Math|Boolean|ANDBoolean (>= _x 0) (>= _y 0) (< _x _boardheight) (< _y _boardheight)) ; 0~8以外は盤面外
    ;[1 1 1] 移動先に駒があるかどうか
    (if (Utilities|IsValid (Utilities|Array|Get(acopy) (Variables|Default|GetcurrentKomaPositionList) (Utilities|PointtoGridIndex point)))
      ;[1 1 1] 移動先に味方の駒がいた場合のリスト
      (Utilities|Array|Add (Variables|Default|GetblockGridList) point)
      (else
        ;[1 1 1] selectedKomaが移動できるリスト
        (Utilities|Array|Add (Variables|Default|GetkomaRangeList) point)))))

(fn PhaseChange
  (params (nextPhase :type Phase%20Enum :default "NewEnumerator0"))
  (Variables|Default|SetcurrentPhase nextPhase))

(fn InMovingRange
  (params (B :type Object%20Object%20Reference))
  (bind _selectedkoma (Variables|Default|GetselectedKoma))
  (for _array_element (Variables|Default|GetinRangeGridList)
    (if (== _array_element B)
      (Variables|/Game/ブループリント/koma/koma_BP.koma_BP_C|SetgridPosition _selectedkoma (Variables|/Game/Grid_BP.Grid_BP_C|GetgridPosition _array_element))
      (Default|Move _selectedkoma)
      (Variables|Default|SetisMoving true)))
  (CallFunction|PhaseChange "NewEnumerator1"))

(fn KillingKoma
  (params (koma :type Koma%20BP%20Object%20Reference))
  ;[1 1 1] 消す前処理
  (Utilities|Array|SetArrayElem (Variables|Default|GetcurrentKomaPositionList) (Variables|/Game/ブループリント/koma/koma_BP.koma_BP_C|GetgridIndex koma) 0)
  (Actor|DestroyActor koma))

(fn InAttackRange
  (params (InputPin :type Grid%20BP%20Object%20Reference))
  (for _array_element (Variables|Default|GetinRangeGridList)
    (if (== _array_element InputPin)
      (bind _kill (Default|Attack (Variables|Default|GetselectedKoma) (Variables|/Game/Grid_BP.Grid_BP_C|GetgridNum _array_element)))
      (if _kill
        (Variables|Default|SetisAttack true))))
  (for _array_element_2 (Variables|Default|GetcurrentBlockGridList)
    (if (== _array_element_2 InputPin)
      (bind _kill_2 (Default|Attack (Variables|Default|GetselectedKoma) (Variables|/Game/Grid_BP.Grid_BP_C|GetgridNum _array_element_2)))
      (if _kill_2
        (Variables|Default|SetisAttack true))))
  (CallFunction|PhaseChange "NewEnumerator1"))

(fn TurnChange
  (params (nextTurn :type Turn%20Enum :default "NewEnumerator2"))
  (Variables|Default|SetcurrentTurn nextTurn))