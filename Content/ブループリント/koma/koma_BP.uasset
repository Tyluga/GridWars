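; Board piece (koma) Blueprint for a two-player, turn-based grid game, coordinated by GameManager_BP.
; It converts world position to a grid cell, registers itself in the manager's flattened board array and derives facing from player tags.
; Clicks report to the manager by phase, with a turn check in Main, and Tick enlarges the selected piece.
; Move snaps to the grid position, while Attack rejects allies and has the manager kill enemies.
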(event EventBeginPlay
  ;[1 1 1] ゲームマネージャーを取得
  (bind _outactors (Actor|GetAllActorsOfClass "/Game/ブループリント/GameManager_BP.GameManager_BP_C"))
  (Variables|Default|SetGameManager (Utilities|Array|Get(acopy) _outactors))
  ;[1 1 1] 位置情報をマス目として保存する
  (CallFunction|MakeGridPostiion)
  ;[1 1 1] この駒の向きを取得
  (CallFunction|ChoiceDirection))

(event MouseInput|EventActorOnClicked
  (params (ButtonPressed :type Key%20Structure))
  (bind _self self)
  (bind _gamemanager (Variables|Default|GetGameManager))
  ;[1 1 1] クリックされたとき
  (switch Utilities|FlowControl|Switch|SwitchonPhase (Variables|/Game/ブループリント/GameManager_BP.GameManager_BP_C|GetcurrentPhase (Variables|Default|GetGameManager))
    (:NewEnumerator1
      (if (Utilities|SearchEnuminTags (Variables|/Game/ブループリント/GameManager_BP.GameManager_BP_C|GetcurrentTurn (Variables|Default|GetGameManager)))
        (Variables|/Game/ブループリント/GameManager_BP.GameManager_BP_C|SetselectedKoma _gamemanager _self)
        (Default|SelectedKomaEvent _gamemanager _self :!label _label)
        (else
          (Development|PrintString "敵の駒です" true true "(R=1.000000,G=0.163765,B=0.000000,A=1.000000)"))))
    (:NewEnumerator5
      (goto _label))))

(event EventTick
  (params (DeltaSeconds :type Float%20%28single-precision%29))
  (bind _defaultsceneroot (Variables|コンポーネント|GetDefaultSceneRoot))
  (bind _gamemanager (Variables|Default|GetGameManager))
  ;[1 0.09206 0] もっと良い処理があるはずなのでいずれ変更する
  ;;[1 1 1] 選択されていたら大きくなる
  (switch Utilities|FlowControl|Switch|SwitchonPhase (Variables|/Game/ブループリント/GameManager_BP.GameManager_BP_C|GetcurrentPhase _gamemanager)
    (:NewEnumerator1
      (Transformation|SetWorldScale3D _defaultsceneroot "1.000000,1.000000,1.000000" :!label _label))
    (:NewEnumerator7
      (if (== (Variables|/Game/ブループリント/GameManager_BP.GameManager_BP_C|GetselectedKoma _gamemanager) self) :!label _label_2
        (Transformation|SetWorldScale3D _defaultsceneroot "1.500000,1.500000,1.000000")))
    (:NewEnumerator4
      (goto _label_2))
    (:NewEnumerator5
      (goto _label_2))
    (:NewEnumerator6
      (goto _label))))

(fn ConstructionScript)

(fn Move
  (bind _gridposition (Variables|Default|GetgridPosition))
  (bind _gamemanager (Variables|Default|GetGameManager))
  (bind _gridscale (Variables|/Game/ブループリント/GameManager_BP.GameManager_BP_C|GetGridScale _gamemanager))
  (Transformation|SetActorLocation (Math|Vector|MakeVector (* (.x _gridposition) _gridscale) (* (.y _gridposition) _gridscale) (.z (Transformation|GetActorLocation))) false false)
  (CallFunction|MakeGridPostiion))

(fn ChoiceDirection
  (if (Utilities|Array|ContainsItem (Variables|Actor|GetTags) "Player2")
    (Variables|Default|Setdirection -1)
    (else
      (Variables|Default|Setdirection 1))))

(fn MakeGridPostiion
  (bind _returnvalue (Transformation|GetActorLocation))
  (bind _gamemanager (Variables|Default|GetGameManager))
  (bind _gamemanager_2 (Variables|Default|GetGameManager))
  (bind _gridscale (Variables|/Game/ブループリント/GameManager_BP.GameManager_BP_C|GetGridScale _gamemanager))
  (Variables|Default|SetgridPosition (Utilities|Struct|MakeIntPoint (Math|Float|Truncate (/ (.x _returnvalue) _gridscale)) (Math|Float|Truncate (/ (.y _returnvalue) _gridscale))))
  ;[1 1 1] ゲームマネージャーにこの駒の情報を渡す
  (Utilities|Array|SetArrayElem (Variables|/Game/ブループリント/GameManager_BP.GameManager_BP_C|GetcurrentKomaPositionList _gamemanager_2) (+ (* (.x (Variables|Default|GetgridPosition)) (Variables|/Game/ブループリント/GameManager_BP.GameManager_BP_C|GetBoardWidth _gamemanager_2)) (.y (Variables|Default|GetgridPosition))) self true)
  ;[1 1 1] 前にいたところは何も無しをいれる
  (if (== (Variables|Default|GetgridIndex) -1)
    _
    (else
      (Utilities|Array|SetArrayElem (Variables|/Game/ブループリント/GameManager_BP.GameManager_BP_C|GetcurrentKomaPositionList (Variables|Default|GetGameManager)) (Variables|Default|GetgridIndex) 0)))
  (Variables|Default|SetgridIndex (+ (* (.x (Variables|Default|GetgridPosition)) (Variables|/Game/ブループリント/GameManager_BP.GameManager_BP_C|GetBoardWidth _gamemanager_2)) (.y (Variables|Default|GetgridPosition)))))

(fn Attack
  (params (gridIndex :type Integer))
  (bind _gamemanager (Variables|Default|GetGameManager))
  (bind _currentkomapositionlist (Variables|/Game/ブループリント/GameManager_BP.GameManager_BP_C|GetcurrentKomaPositionList _gamemanager))
  (bind _output (Utilities|Array|Get(acopy) _currentkomapositionlist gridIndex))
  (Utilities|IsValid _output
    (:Is%20Valid
      (if (Actor|ActorHasTag _output (Utilities|Array|Get(acopy) (Variables|Actor|GetTags)))
        (Development|PrintString "味方の駒です" true true "(R=1.000000,G=0.000000,B=0.213972,A=1.000000)")
        (else
          (Default|KillingKoma _gamemanager _output)
          (return true))))
    (:Is%20Not%20Valid
      (return false))))