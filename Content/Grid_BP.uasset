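; Board tile actor for a phase-based grid game that highlights movement and attack areas and forwards clicks to GameManager_BP as selections.
; On BeginPlay it derives its cell from world position and registers itself in the manager's flattened GridList.
; Tick colors a dynamic material from the current phase and IsRange/IsBlock flags: blue or yellow in Moving, red in Attack, otherwise white.
; Phases other than Moving and Attack also clear both flags.
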(event EventBeginPlay
  (bind _returnvalue (Transformation|GetActorLocation))
  (Utilities|FlowControl|Sequence
    (:then_0
      ;[1 1 1] ゲームマネージャーの取得
      (bind _outactors (Actor|GetAllActorsOfClass "/Game/ブループリント/GameManager_BP.GameManager_BP_C"))
      (Variables|Default|SetGameManager (Utilities|Array|Get(acopy) _outactors))
      ;[1 1 1] ダイナミックマテリアルの生成
      (bind _asmaterial_instance_dynamic (Utilities|Casting|CastToMaterialInstanceDynamic (Rendering|Material|GetMaterial (Variables|Default|GetPlane) 0)))
      (Variables|Default|SetdynamicMaterial _asmaterial_instance_dynamic))
    (:then_1
      ;[1 1 1] ゲームマネージャにこのグリッドを記録する
      (Variables|Default|SetgridPosition (Utilities|Struct|MakeIntPoint (Math|Float|Truncate (/ (.x _returnvalue) (Variables|/Game/ブループリント/GameManager_BP.GameManager_BP_C|GetGridScale (Variables|Default|GetGameManager)))) (Math|Float|Truncate (/ (.y _returnvalue) (Variables|/Game/ブループリント/GameManager_BP.GameManager_BP_C|GetGridScale (Variables|Default|GetGameManager))))))
      (Variables|Default|SetgridNum (+ (* (Math|Float|Truncate (/ (.x _returnvalue) (Variables|/Game/ブループリント/GameManager_BP.GameManager_BP_C|GetGridScale (Variables|Default|GetGameManager)))) (Variables|/Game/ブループリント/GameManager_BP.GameManager_BP_C|GetBoardWidth (Variables|Default|GetGameManager))) (Math|Float|Truncate (/ (.y _returnvalue) (Variables|/Game/ブループリント/GameManager_BP.GameManager_BP_C|GetGridScale (Variables|Default|GetGameManager))))))
      (Utilities|Array|SetArrayElem (Variables|/Game/ブループリント/GameManager_BP.GameManager_BP_C|GetgridList (Variables|Default|GetGameManager)) (+ (* (Math|Float|Truncate (/ (.x _returnvalue) (Variables|/Game/ブループリント/GameManager_BP.GameManager_BP_C|GetGridScale (Variables|Default|GetGameManager)))) (Variables|/Game/ブループリント/GameManager_BP.GameManager_BP_C|GetBoardWidth (Variables|Default|GetGameManager))) (Math|Float|Truncate (/ (.y _returnvalue) (Variables|/Game/ブループリント/GameManager_BP.GameManager_BP_C|GetGridScale (Variables|Default|GetGameManager))))) self true))))

(event EventTick
  (params (DeltaSeconds :type Float%20%28single-precision%29))
  ;[1 1 1] 光らせる
  (switch Utilities|FlowControl|Switch|SwitchonPhase (Variables|/Game/ブループリント/GameManager_BP.GameManager_BP_C|GetcurrentPhase (Variables|Default|GetGameManager))
    (:NewEnumerator0
      ;;[1 1 1] 範囲外またはAttack、Moving以外
      (Variables|Default|SetisRange false :!label _label)
      (Variables|Default|SetisBlock false)
      (Rendering|Material|SetVectorParameterValue (Variables|Default|GetdynamicMaterial) "colorParam" "(R=1.000000,G=1.000000,B=1.000000,A=1.000000)" :!class /Script/Engine.MaterialInstanceDynamic :!label _label_2))
    (:NewEnumerator1
      (goto _label))
    (:NewEnumerator7
      (goto _label))
    (:NewEnumerator4
      ;;[0.1668 0.1568 1] 移動範囲
      (if (Variables|Default|GetisRange)
        (Rendering|Material|SetVectorParameterValue (Variables|Default|GetdynamicMaterial) "colorParam" "(R=0.000000,G=0.270360,B=1.000000,A=1.000000)" :!class /Script/Engine.MaterialInstanceDynamic)
        (else
          ;;[1 0.8122 0.2207] ブロック範囲
          (if (Variables|Default|GetisBlock)
            (Rendering|Material|SetVectorParameterValue (Variables|Default|GetdynamicMaterial) "colorParam" "(R=1.000000,G=0.885502,B=0.000000,A=1.000000)" :!class /Script/Engine.MaterialInstanceDynamic)
            (else
              (goto _label_2))))))
    (:NewEnumerator5
      ;;[1 0.1281 0.1281] 攻撃範囲
      (if (Variables|Default|GetisRange)
        _
        (elif (Variables|Default|GetisBlock)
          _
          (else
            (goto _label_2))))
      (Rendering|Material|SetVectorParameterValue (Variables|Default|GetdynamicMaterial) "colorParam" "(R=1.000000,G=0.066757,B=0.000000,A=1.000000)" :!class /Script/Engine.MaterialInstanceDynamic))
    (:NewEnumerator6
      (goto _label))))

(event MouseInput|EventActorOnClicked
  (params (ButtonPressed :type Key%20Structure))
  ;[1 1 1] グリッドクリック時
  (Default|SelectedGridEvent (Variables|Default|GetGameManager) self))

(fn ConstructionScript
  (Rendering|Material|CreateDynamicMaterialInstance (Variables|Default|GetPlane) 0 "/Game/マテリアル（仮）/Grid_Mat.Grid_Mat" :!class /Script/Engine.PrimitiveComponent))